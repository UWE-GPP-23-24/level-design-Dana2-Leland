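; BP_OverstimulationLight is a light Blueprint whose spotlight endlessly animates its intensity and changes color.
; From BeginPlay, a timeline drives the SpotLight's intensity on each update.
; When the timeline finishes, it gives the light a random hue and restarts itself through the LoopLight event, so each cycle after the first begins with a newly randomized color.
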(event Custom|loopLight
  (bind _newtrack_0 (Timeline|Timeline PlayFromStart)
    (:Update
      (Rendering|Components|Light|SetIntensity (Variables|Default|GetSpotLight) _newtrack_0))
    (:Finished
      (CallFunction|RandomColor)
      (CallFunction|LoopLight))))

(event Custom|randomColor
  (Class|KismetMathLibrary|LinearColorSetRandomHue (Variables|Default|GetNew%20Light%20Color))
  (Rendering|Components|Light|SetLightColor (Variables|Default|GetSpotLight) (Variables|Default|GetNew%20Light%20Color) true))

(event EventBeginPlay
  (CallFunction|LoopLight))

(fn ConstructionScript)