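; AI controller for the no-gravity Boom Bot that turns perception of the player into the bot's target.
; It caches the controlled bot on BeginPlay and calls its SetTarget directly from AI Perception events.
; Any perception update on the player sets it as the target, without checking whether the stimulus was sensed or lost.
; The target clears only when perception forgets the player.
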(event OnTargetPerceptionUpdated(AIPerception)
  (params (Actor :type Actor%20Object%20Reference) (Stimulus :type AI%20Stimulus%20Structure))
  ;[0.4491 0.8591 1] Detection
  ;;[0.4491 0.8591 1] Check to see if we have seen the player
  (bind _asbp_player_character (Utilities|Casting|CastToBP_PlayerCharacter Actor))
  (Default|SetTarget (Variables|Default|GetAs%20BP%20Boom%20Bot%20No%20Gravity) _asbp_player_character))

(event OnTargetPerceptionForgotten(AIPerception)
  (params (Actor :type Actor%20Object%20Reference))
  ;[0.4491 0.8591 1] Detection
  ;;[0.4491 0.8591 1] Check to see if we have lost the player
  (Utilities|Casting|CastToBP_PlayerCharacter Actor)
  (Default|SetTarget (Variables|Default|GetAs%20BP%20Boom%20Bot%20No%20Gravity)))

(event EventBeginPlay
  ;[0.4491 0.8591 1] Cache ref to bot
  (bind _asbp_boom_bot_no_gravity (Utilities|Casting|CastToBP_BoomBotNoGravity (Pawn|GetControlledPawn)))
  (Variables|Default|SetAs%20BP%20Boom%20Bot%20No%20Gravity _asbp_boom_bot_no_gravity))

(fn ConstructionScript)