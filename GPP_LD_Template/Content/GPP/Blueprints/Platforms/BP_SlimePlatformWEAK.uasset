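; BP_SlimePlatformWEAK is a freezable slime platform that bounces characters entering its box trigger.
; On begin play it applies a dynamic material instance to the mesh and hands it to the freezable component, then initializes freeze status.
; On overlap it launches the character along the mesh's up vector by a launch multiplier, overriding Z velocity only.
; While frozen, the launch velocity drops to zero.
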(event OnComponentBeginOverlap(Box)
  (params (OverlappedComponent :type Primitive%20Component%20Object%20Reference) (OtherActor :type Actor%20Object%20Reference) (OtherComp :type Primitive%20Component%20Object%20Reference) (OtherBodyIndex :type Integer) (bFromSweep :type Boolean) (SweepResult :type Hit%20Result%20Structure%20%28by%20ref%29))
  (bind _ascharacter (Utilities|Casting|CastToCharacter OtherActor))
  ;[0.4491 0.8591 1] Try to launch character if not frozen
  (Character|LaunchCharacter _ascharacter (* (Math|Vector|GetUpVector (Variables|Default|GetPlatformMesh)) (select (Default|GetIsFrozen (Variables|Default|GetBP_FreezableComponent)) 0.0 (Variables|Default|GetLaunchMultiplier))) false true))

(event EventBeginPlay
  (bind _platformmesh (Variables|Default|GetPlatformMesh))
  (bind _bp_freezablecomponent (Variables|Default|GetBP_FreezableComponent))
  ;[0.4491 0.8591 1] Create material instance
  (bind _returnvalue (Rendering|Material|CreateDynamicMaterialInstance (Rendering|Material|GetMaterial _platformmesh 0) "None" "None" :!class /Script/Engine.KismetMaterialLibrary))
  (Rendering|Material|SetMaterial _platformmesh 0 _returnvalue)
  ;;[0.4491 0.8591 1] Initialise the freezable component
  (Default|InitMaterial _bp_freezablecomponent (Utilities|Array|MakeArray _returnvalue))
  (Default|InitFreezeStatus _bp_freezablecomponent))

(fn ConstructionScript)