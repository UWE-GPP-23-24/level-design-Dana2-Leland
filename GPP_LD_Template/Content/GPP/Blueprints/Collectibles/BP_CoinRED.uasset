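; BP_CoinRED is a spinning collectible coin that starts hidden, with mesh collision disabled; nothing in this Blueprint re-enables it.
; Tick yaws the actor by RotateSpeed.
; Collect adds the coin's score through GM_Gameplay, spawns a Niagara effect and calls ChangeCoinCount before destroying the actor.
; ChangeCoinCount finds BP_Sign with GetActorOfClass and passes its coin count minus one to OnCoin.
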(event EventBeginPlay
  (bind _mesh (Variables|Default|GetMesh))
  (Collision|SetCollisionEnabled _mesh "NoCollision")
  (Rendering|SetVisibility _mesh false false))

(event EventTick
  (params (DeltaSeconds :type Float%20%28single-precision%29))
  ;[0.4491 0.8591 1] Rotate Coin
  (Class|Actor|AddActorWorldRotation (Math|Rotator|MakeRotator 0.0 0.0 (* DeltaSeconds (Variables|Default|GetRotate%20Speed)))))

(event EventCollect
  (params (Collector :type BP%20Player%20Character%20Object%20Reference))
  ;[0.4491 0.8591 1] Collect Coin
  ;;[0.4491 0.8591 1] Add score
  (bind _asgm_gameplay (Utilities|Casting|CastToGM_Gameplay (Game|GetGameMode)))
  (Default|AddScore _asgm_gameplay (.scorevalue (Variables|Default|GetData)))
  ;;[0.4491 0.8591 1] Spawn particle
  (Niagara|SpawnSystematLocation "/Game/GPP/Particles/NS_CoinCollect.NS_CoinCollect" (Transformation|GetWorldLocation (Variables|Default|GetMesh)))
  (CallFunction|ChangeCoinCount)
  ;;[0.4491 0.8591 1] Destroy self
  (Actor|DestroyActor))

(fn ConstructionScript)

(fn ChangeCoinCount
  (bind _returnvalue (Actor|GetActorOfClass "/Game/GPP/Blueprints/Dana_UPDATES/Sign/BP_Sign.BP_Sign_C"))
  (Default|OnCoin _returnvalue (- (Variables|/Game/GPP/Blueprints/Dana_UPDATES/Sign/BP_Sign.BP_Sign_C|GetBPSignCoin _returnvalue) 1))
  (return (- (Variables|/Game/GPP/Blueprints/Dana_UPDATES/Sign/BP_Sign.BP_Sign_C|GetBPSignCoin _returnvalue) 1)))